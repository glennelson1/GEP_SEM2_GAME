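; BP_PickUp is a collectable pickup actor that counts toward the game's remaining collectables.
; When its M_Collider component begins an overlap, it decrements CollectablesLeft on BP_MyGameMode, without checking which actor touched it.
; It then adds a new Collectablwidget to the viewport, plays an explosion particle and sound at its location, and destroys itself.
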(event OnComponentBeginOverlap(m_Collider)
  (params (OverlappedComponent :type Primitive%20Component%20Object%20Reference) (OtherActor :type Actor%20Object%20Reference) (OtherComp :type Primitive%20Component%20Object%20Reference) (OtherBodyIndex :type Integer) (bFromSweep :type Boolean) (SweepResult :type Hit%20Result%20Structure%20%28by%20ref%29))
  (bind _returnvalue (Transformation|GetActorLocation))
  (bind _asbp_my_game_mode (Utilities|Casting|CastToBP_MyGameMode (Game|GetGameMode)))
  (bind _result (Math|Integer|DecrementInt (Variables|/Game/-GameAssets/BP_MyGameMode.BP_MyGameMode_C|GetCollectables_Left _asbp_my_game_mode))
    (:%20%20
      (Variables|/Game/-GameAssets/BP_MyGameMode.BP_MyGameMode_C|SetCollectables_Left _asbp_my_game_mode _result)
      (bind _returnvalue_2 (UserInterface|CreateWidget "/Game/-GameAssets/Collectablwidget.Collectablwidget_C"))
      (UserInterface|Viewport|AddtoViewport _returnvalue_2 0)
      (Effects|SpawnEmitteratLocation "/Game/StarterContent/Particles/P_Explosion.P_Explosion" _returnvalue)
      (Audio|PlaySoundatLocation "/Game/-SoundEffects/mixkit-short-explosion-1694.mixkit-short-explosion-1694" _returnvalue "0, 0, 0" 1.0 1.0 0.0 0 0 0)
      (Actor|DestroyActor))))

(event EventBeginPlay)

(event Collision|EventActorBeginOverlap
  (params (OtherActor :type Actor%20Object%20Reference)))

(event EventTick
  (params (DeltaSeconds :type Float%20%28single-precision%29)))

(fn ConstructionScript)